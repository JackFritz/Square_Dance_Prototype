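; BP_FarJumpPad is a jump pad that launches the player along its Arrow component's forward vector.
; A Box overlap by BP_Player plays a timeline that tilts the whole actor's pitch.
; When the timeline finishes, a DoOnce triggers the player's Jump, then after a short delay adds launch velocity via LaunchCharacter and resets the gate.
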(event `self.Box.OnComponentBeginOverlap`
  (params (OverlappedComponent :type "PrimitiveComponent Object Reference") (OtherActor :type "Actor Object Reference") (OtherComp :type "PrimitiveComponent Object Reference") (OtherBodyIndex :type Integer) (bFromSweep :type Boolean) (SweepResult :type "HitResult Structure (by ref)"))
  (bind (_returnvalue_roll _returnvalue_pitch _returnvalue_yaw) (`KismetMathLibrary.BreakRotator` (`self.K2_GetActorRotation`)))
  (bind _asbp_player (cast `/Game/Blueprints/BP_Player` OtherActor))
  (bind (_direction _launch_track) (`Timeline|JumpPadAnimation TL` :!via `PlayFromStart`)
    (:`Update`
      (`self.K2_SetActorRotation` (`KismetMathLibrary.MakeRotator` _returnvalue_roll (`KismetMathLibrary.Lerp` -10.0 10.0 _launch_track) _returnvalue_yaw)))
    (:`Finished`
      (`/Engine/EditorBlueprintResources/StandardMacros.DoOnce` false :!label _label
        (:`Completed`
          (`Character.Jump` _asbp_player)
          (`KismetSystemLibrary.Delay` 0.2)
          (`Character.LaunchCharacter` _asbp_player (* (`SceneComponent.GetForwardVector` (`self.Arrow`)) 3000.0) false false)
          (goto _label :!via `Reset`))))))

(fn `UserConstructionScript`)